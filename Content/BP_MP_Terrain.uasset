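; Terrain generator Blueprint that sets up procedural, tiled terrain of mountains and low hills on BeginPlay.
; A low-frequency simplex noise selects, with sine-eased falloff, between domain-warped inverted ridged-multifractal mountains and scaled FBM hills.
; That noise graph feeds both height and biome blend in the CG terrain config, alongside tile, material and two-LOD settings, with collision only on the near LOD.
; A radial island-style mask module is left unconnected.
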(event EventBeginPlay
  (bind _self self)
  (bind _self_2 self)
  (bind _self_3 self)
  (bind _self_4 self)
  (bind _returnvalue (Class|UFNBlueprintFunctionLibrary|CreateFractalNoiseGenerator _self_2 "FractalSimplex" 326541 1e-05 0.5 "InterpLinear" "FBM" 4 1.7))
  (bind _returnvalue_2 (Class|UFNBlueprintFunctionLibrary|CreateFractalNoiseGenerator _self_4 "FractalSimplex" 2147483647 1e-06 0.5 "InterpLinear" "FBM" 1 1.7))
  (bind _returnvalue_3 (Class|UFNBlueprintFunctionLibrary|CreateFractalNoiseGenerator _self "FractalSimplex" 12345 7e-06 0.5 "InterpLinear" "RigidMulti" 9 1.7))
  (bind _returnvalue_4 (Class|UFNBlueprintFunctionLibrary|CreateScaleBiasModule _self_2 _returnvalue 0.5 -0.5))
  (bind _returnvalue_5 (Class|UFNBlueprintFunctionLibrary|CreateScaleBiasModule _self _returnvalue_3 -1.0 0.0))
  (bind _returnvalue_6 (Class|UFNBlueprintFunctionLibrary|CreateWarpModule _self _returnvalue_5 _returnvalue_5 3e+04 "Two"))
  (bind _returnvalue_7 (Class|UFNBlueprintFunctionLibrary|CreateSelectModule _self_3 _returnvalue_6 _returnvalue_4 _returnvalue_2 "SineInOut" 0.5 0.0 4))
  (Class|CGTerrainManager|SetupTerrainGenerator (Utilities|Struct|MakeCGTerrainConfig _returnvalue_7 _returnvalue_7 48 48 2e+02 1.5e+04 0 1.0 1.0 1e+01 0.1 0.0 10 1 1 (Math|Timespan|MakeTimespan 0 0 0 5) 0.01 "/CashGen/TerrainMaterial.TerrainMaterial" false 0 false (Utilities|Array|MakeArray (Utilities|Struct|MakeCGLODConfig 5.0 4 1 true) (Utilities|Struct|MakeCGLODConfig 5.0 8 8)))))

(fn ConstructionScript)
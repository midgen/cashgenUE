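; BP_World is a world actor that builds a procedural noise graph on BeginPlay and passes it to SetupWorld, likely for terrain.
; A warped low-octave FBM selector blends a flat constant with domain-warped ridged multifractal simplex noise.
; A radial module with a soft falloff blends that result with a lower constant around an offset origin.
; OnDrawComplete only prints a debug message.
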(event EventBeginPlay
  (bind _self self)
  (bind _self_2 self)
  (bind _returnvalue (Class|UFNBlueprintFunctionLibrary|CreateFractalNoiseGenerator _self "FractalSimplex" 12345 5e-05 0.5 "InterpLinear" "RigidMulti" 8 1.7))
  (bind _returnvalue_2 (Class|UFNBlueprintFunctionLibrary|CreateFractalNoiseGenerator _self "FractalSimplex" 32647 0.0001 0.5 "InterpLinear" "FBM" 2 1.7))
  (Class|CGWorld|SetupWorld (Class|UFNBlueprintFunctionLibrary|CreateRadialModule _self_2 (Class|UFNBlueprintFunctionLibrary|CreateConstantModule _self_2 -5e+01) (Class|UFNBlueprintFunctionLibrary|CreateSelectModule _self (Class|UFNBlueprintFunctionLibrary|CreateConstantModule _self -1.0) (Class|UFNBlueprintFunctionLibrary|CreateWarpModule _self _returnvalue _returnvalue 6e+03 "Two") (Class|UFNBlueprintFunctionLibrary|CreateWarpModule _self _returnvalue_2 _returnvalue_2 2e+03 "Two") "CircularInOut" 0.5 0.0 4) "CircularIn" "5000.000000,0.000000,0.000000" 0.0 2e+03 4)))

(event EventOnDrawComplete
  (Development|PrintString "Draw Complete!"))

(fn ConstructionScript)